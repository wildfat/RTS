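; Player state Blueprint that handles a player joining a team and requests that player's pawn spawn.
; On ROC_PlayerJoined it stores the team name in DSS_GameInstance, which then sets the default pawn.
; It passes that pawn and the transform of the first BP_SpawnPoint found to ROSSetPlayerToSpawn on the first local DSS_PlayerController.
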(event Custom|ROC_PlayerJoined
  (params (TeamName :type Name))
  (bind _asdss_game_instance (Utilities|Casting|CastToDSS_GameInstance (Game|GetGameInstance)))
  (Variables|/Game/Blueprints/Logics/DSS_GameInstance.DSS_GameInstance_C|SetTeamName _asdss_game_instance TeamName)
  (Default|SetDefaultPawn _asdss_game_instance)
  (bind _outactors (Actor|GetAllActorsOfClass "/Game/Blueprints/Enviroments/BP_SpawnPoint.BP_SpawnPoint_C"))
  (bind _asdss_player_controller (Utilities|Casting|CastToDSS_PlayerController (Game|GetPlayerController 0)))
  (Default|ROSSetPlayertoSpawn _asdss_player_controller (Variables|/Game/Blueprints/Logics/DSS_GameInstance.DSS_GameInstance_C|GetDefaultPawn _asdss_game_instance) (Transformation|GetActorTransform (Utilities|Array|Get(acopy) _outactors)) _asdss_player_controller))

(fn ConstructionScript)