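; HUD Blueprint that draws a drag-selection box and selects the local player's units.
; While drawing, DrawHUD stretches a brick texture from the click to the mouse and sorts the corners into min/max bounds.
; It projects every locally commanded BP_MasterUnit to screen space each frame and tests it against the box.
; Units inside join SelectedActors and get a selected message; units outside are deselected unless MultipleSelection is on.
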(event EventDrawHUD
  (params (SizeX :type Integer) (SizeY :type Integer))
  (bind _returnvalue (Game|GetPlayerController 0))
  (bind _clickedlocation (Variables|Default|GetClickedLocation))
  (bind (_locationx _locationy) (Game|Player|GetMousePosition _returnvalue))
  (bind (_x _y) (Math|Vector2D|BreakVector2D _clickedlocation))
  (Variables|Default|SetScreenResolution (Math|Vector2D|MakeVector2D (Math|Conversions|ToFloat(Integer) SizeX) (Math|Conversions|ToFloat(Integer) SizeY)))
  (if (Variables|Default|GetIsDrawing)
    (Variables|Default|SetCurrentMouseLocation (Math|Vector2D|MakeVector2D _locationx _locationy))
    (Canvas|DrawTexture "/Game/StarterContent/Textures/T_Brick_Clay_New_D.T_Brick_Clay_New_D" _x _y (.X (Math|Vector2D|BreakVector2D (- (Variables|Default|GetCurrentMouseLocation) _clickedlocation))) (.Y (Math|Vector2D|BreakVector2D (- (Variables|Default|GetCurrentMouseLocation) _clickedlocation))) 0.0 0.0 0.0 0.0 "(R=1.000000,G=1.000000,B=1.000000,A=1.000000)")
    (CallFunction|CheckDragBoxDimension)
    (bind _outactors (Actor|GetAllActorsOfClass "/Game/MasterBlueprints/Units/BP_MasterUnit.BP_MasterUnit_C"))
    (for _array_element _outactors
      (if (Pawn|IsLocallyControlled (Variables|/Game/MasterBlueprints/Units/BP_MasterUnit.BP_MasterUnit_C|GetLocalCommander _array_element))
        (bind _isindragbox (CallFunction|IsActorinDragBox (.ScreenLocation (Class|PlayerController|ProjectWorldLocationtoScreen (Game|GetPlayerController 0) (Transformation|GetActorLocation _array_element) false))))
        (if _isindragbox
          (CallFunction|ActorIsinDragbox _array_element)
          (elif (not (Variables|Default|GetMultipleSelection))
            (CallFunction|ActorIsNotinDragBox _array_element)))))))

(fn ConstructionScript)

(fn CheckDragBoxDimension
  (bind _clickedlocation (Variables|Default|GetClickedLocation))
  (bind _currentmouselocation (Variables|Default|GetCurrentMouseLocation))
  (bind (_x _y) (Math|Vector2D|BreakVector2D _clickedlocation))
  (bind (_x_2 _y_2) (Math|Vector2D|BreakVector2D _currentmouselocation))
  (Utilities|FlowControl|Sequence
    (:then_0
      (if (>= (- _x_2 _x) 0.0)
        (Variables|Default|SetXMin _x)
        (Variables|Default|SetXMax _x_2)
        (else
          (Variables|Default|SetXMin _x_2)
          (Variables|Default|SetXMax _x))))
    (:then_1
      (if (>= (- _y_2 _y) 0.0)
        (Variables|Default|SetYMin _y)
        (Variables|Default|SetYMax _y_2)
        (else
          (Variables|Default|SetYMin _y_2)
          (Variables|Default|SetYMax _y))))))

(fn IsActorinDragBox
  (params (InActor2DVector :type Vector%202D%20Structure))
  (bind (_x _y) (Math|Vector2D|BreakVector2D InActor2DVector))
  (return (Math|Boolean|ANDBoolean (>= _x (Variables|Default|GetXMin)) (<= _x (Variables|Default|GetXMax)) (>= _y (Variables|Default|GetYMin)) (<= _y (Variables|Default|GetYMax)))))

(fn ActorIsinDragbox
  (params (InActor :type Actor%20Object%20Reference))
  (bind _selectedactors (Variables|Default|GetSelectedActors))
  (if (not (Utilities|Array|ContainsItem _selectedactors InActor))
    (Utilities|Array|Add _selectedactors InActor)
    (Class|DSSInterface|ImSelected(Message) InActor)))

(fn ActorIsNotinDragBox
  (params (InActor :type Actor%20Object%20Reference))
  (bind _selectedactors (Variables|Default|GetSelectedActors))
  (if (Utilities|Array|ContainsItem _selectedactors InActor)
    (Class|DSSInterface|ImNotSelected(Message) InActor)
    (Utilities|Array|RemoveItem _selectedactors InActor)))