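; RTS-style camera pawn that orbits, zooms and glides to a focused actor.
; A 0.2-second delay separates holds, which enable axis-driven rotation, from clicks, which trace under the cursor to set FocusedActor.
; Tick clamps pitch and, while focusing, lerps from the current location to the actor using a float curve over CurveLenght seconds.
; Zoom adjusts spring arm length without limits; a preset FocusedActor gets focus one second after BeginPlay.
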(event EventBeginPlay
  (Utilities|FlowControl|Delay 1.0)
  (Utilities|IsValid (Variables|Default|GetFocusedActor)
    (:Is%20Valid
      (Variables|Default|SetFocus true))))

(event EventTick
  (params (DeltaSeconds :type Float%20%28single-precision%29))
  (CallFunction|CameraLimits)
  (if (Variables|Default|GetFocus)
    (CallFunction|MovetoFoFocusedActor (Variables|Default|GetFocusedActor))
    (bind _output_get (Variables|Default|SetElapsedTime (+ DeltaSeconds (Variables|Default|GetElapsedTime))))
    (if (> _output_get (Variables|Default|GetCurveLenght))
      (Variables|Default|SetElapsedTime 0.0)
      (Variables|Default|SetFocus false))))

(event Input|ActionEvents|InputActionClick
  (params (Key :type Key%20Structure))
  (:Pressed
    (Utilities|FlowControl|Delay 0.2)
    (CallFunction|HandleMouseClick Key))
  (:Released
    (Variables|Default|SetClickHeld false)))

(event Input|ActionEvents|InputActionZoomIn
  (params (Key :type Key%20Structure))
  ;[1 1 1] Zoom
  (:Pressed
    (CallFunction|Zoom -2e+01)))

(event Input|ActionEvents|InputActionZoomOut
  (params (Key :type Key%20Structure))
  ;[1 1 1] Zoom
  (:Pressed
    (CallFunction|Zoom 2e+01)))

(event Input|AxisEvents|InputAxisRotateHorizontal
  (params (AxisValue :type Float%20%28single-precision%29))
  ;[1 1 1] Rotation
  (if (Variables|Default|GetClickHeld)
    (Class|Actor|AddActorWorldRotation (Math|Rotator|MakeRotator 0.0 0.0 (* AxisValue (Variables|Default|GetRotationSpeed))))))

(event Input|AxisEvents|InputAxisRotateVertical
  (params (AxisValue :type Float%20%28single-precision%29))
  ;[1 1 1] Rotation
  (if (Variables|Default|GetClickHeld)
    (Transformation|AddActorLocalRotation (Math|Rotator|MakeRotator 0.0 (* AxisValue (Variables|Default|GetRotationSpeed)) 0.0) false false)))

(fn ConstructionScript
  (Variables|Default|SetDefayltArmLenght (Variables|/Script/Engine.SpringArmComponent|GetTargetArmLength (Variables|Default|GetSpringArm))))

(fn CheckifClickHitActor
  (bind _returnvalue (Game|GetPlayerController 0))
  (bind _hitresult (Game|Player|GetHitResultUnderCursorbyChannel _returnvalue "TraceTypeQuery1" true))
  (bind (_bblockinghit _binitialoverlap _time _distance _location _impactpoint _normal _impactnormal _physmat _hitactor) (Collision|BreakHitResult _hitresult))
  (return _bblockinghit _hitactor))

(fn HandleMouseClick
  (params (Key :type Key%20Structure))
  (bind _returnvalue (Game|GetPlayerController 0))
  (bind (_bblockinghit _hitactor) (CallFunction|CheckifClickHitActor))
  (bind _returnvalue_2 (Game|Player|IsInputKeyDown _returnvalue Key))
  (if _returnvalue_2
    (Variables|Default|SetClickHeld _returnvalue_2)
    (elif _bblockinghit
      (Variables|Default|SetFocusedActor _hitactor)
      (Variables|Default|SetElapsedTime 0.0)
      (Variables|Default|SetFocus true))))

(fn Zoom
  (params (ZoomSpeed :type Float%20%28single-precision%29))
  (bind _springarm (Variables|Default|GetSpringArm))
  (Variables|/Script/Engine.SpringArmComponent|SetTargetArmLength _springarm (+ (Variables|/Script/Engine.SpringArmComponent|GetTargetArmLength _springarm) ZoomSpeed)))

(fn CameraLimits
  (bind _returnvalue (Transformation|GetActorRotation))
  (bind _ylimitmin (Variables|Default|GetYLimitMin))
  (bind _ylimitmax (Variables|Default|GetYLimitMax))
  (bind _returnvalue_2 (< (.pitch _returnvalue) _ylimitmin))
  (if (or _returnvalue_2 (> (.pitch _returnvalue) _ylimitmax))
    (Transformation|SetActorRotation (Math|Rotator|MakeRotator 0.0 (Math|Float|SelectFloat _ylimitmin _ylimitmax _returnvalue_2) (.yaw _returnvalue)))))

(fn MovetoFoFocusedActor
  (params (Actor :type Actor%20Object%20Reference))
  (Transformation|SetActorLocation (Math|Vector|Lerp(Vector) (Transformation|GetActorLocation) (Transformation|GetActorLocation Actor) (Math|Curves|GetFloatValue (Variables|Default|GetCameraCurve) (/ (Variables|Default|GetElapsedTime) (Variables|Default|GetCurveLenght)))) false false))