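; Basic rifle weapon that auto-fires BP_BasicRifleBullet projectiles at the owning BP_MasterCombat's current enemy.
; ROS_FireWeapon starts a randomly delayed Fire timer, which re-arms after each shot and lapses when the owner moves or lacks a valid enemy.
; Fire solves ballistic launch pitch for gravity, using separate level-ground and height-difference formulas.
; It takes yaw from the owner, adds slight random spread, and spawns the bullet from BulletSpawnBox.
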(event Custom|ROS_FireWeapon
  (if (not (Class|KismetSystemLibrary|TimerExists 0 "Fire"))
    (Utilities|Time|SetTimerbyFunctionName 0 "Fire" (Math|Random|RandomFloatinRange 0.2 0.5))))

(fn ConstructionScript
  (|CallParentFunction))

(fn Fire
  (bind _returnvalue (Math|Random|RandomIntegerinRange -1 1))
  (bind _weaponowner (Variables|Default|GetWeaponOwner))
  (bind _weaponowner_2 (Variables|Default|GetWeaponOwner))
  (bind _bulletspawnbox (Variables|Default|GetBulletSpawnBox))
  (bind _returnvalue_2 (Transformation|GetActorRotation _weaponowner_2))
  (bind _returnvalue_3 (Math|Conversions|ToFloat(Integer) _returnvalue))
  (bind _returnvalue_4 (Transformation|GetWorldTransform _bulletspawnbox))
  (bind _returnvalue_5 (Transformation|GetActorRotation _weaponowner_2))
  (if (== (Math|Vector|VectorLength (Transformation|GetVelocity _weaponowner)) 0.0)
    (bind _asbp_master_combat (Utilities|Casting|CastToBP_MasterCombat _weaponowner))
    (Utilities|IsValid (Variables|/Game/MasterBlueprints/Units/BP_MasterCombat.BP_MasterCombat_C|GetEnemyToFight _asbp_master_combat)
      (:Is%20Valid
        (if (Math|Float|NearlyEqual(Float) (.z (- (Transformation|GetActorLocation _asbp_master_combat) (Transformation|GetActorLocation (Variables|/Game/MasterBlueprints/Units/BP_MasterCombat.BP_MasterCombat_C|GetEnemyToFight _asbp_master_combat)))) 0.0 1e+01)
          (Transformation|SetWorldRotation _bulletspawnbox (Math|Rotator|MakeRotator (.roll _returnvalue_2) (+ (Class|KismetMathLibrary|DegAsin (Math|Float|Absolute(Float) (/ (* (Math|Vector2D|Vector2DLength (- (Math|Vector2D|MakeVector2D (.X (Math|Vector|BreakVector (Transformation|GetActorLocation (Variables|/Game/MasterBlueprints/Units/BP_MasterCombat.BP_MasterCombat_C|GetEnemyToFight _asbp_master_combat)))) (.Y (Math|Vector|BreakVector (Transformation|GetActorLocation (Variables|/Game/MasterBlueprints/Units/BP_MasterCombat.BP_MasterCombat_C|GetEnemyToFight _asbp_master_combat))))) (Math|Vector2D|MakeVector2D (.X (Math|Vector|BreakVector (Transformation|GetActorLocation _asbp_master_combat))) (.Y (Math|Vector|BreakVector (Transformation|GetActorLocation _asbp_master_combat)))))) -9.8e+02) (* 2 (Math|Float|Square 3e+03))))) (Math|Conversions|ToFloat(Integer) (Math|Random|RandomIntegerinRange -1 1))) (+ (.yaw _returnvalue_2) (Math|Conversions|ToFloat(Integer) (Math|Random|RandomIntegerinRange -1 1)))) false false)
          (else
            (Transformation|SetWorldRotation _bulletspawnbox (Math|Rotator|MakeRotator (.roll _returnvalue_5) (+ (Class|KismetMathLibrary|DegAtan (/ (- (Math|Float|Square 3e+03) (Math|Float|Sqrt (- (Math|Float|Square (Math|Float|Square 3e+03)) (* 9.8e+02 (+ (* (Math|Float|Square (Math|Vector2D|Vector2DLength (- (Math|Vector2D|MakeVector2D (.X (Math|Vector|BreakVector (Transformation|GetActorLocation (Variables|/Game/MasterBlueprints/Units/BP_MasterCombat.BP_MasterCombat_C|GetEnemyToFight _asbp_master_combat)))) (.Y (Math|Vector|BreakVector (Transformation|GetActorLocation (Variables|/Game/MasterBlueprints/Units/BP_MasterCombat.BP_MasterCombat_C|GetEnemyToFight _asbp_master_combat))))) (Math|Vector2D|MakeVector2D (.X (Math|Vector|BreakVector (Transformation|GetActorLocation _asbp_master_combat))) (.Y (Math|Vector|BreakVector (Transformation|GetActorLocation _asbp_master_combat))))))) -9.8e+02) (* (* 2.0 (.z (- (Transformation|GetActorLocation _asbp_master_combat) (Transformation|GetActorLocation (Variables|/Game/MasterBlueprints/Units/BP_MasterCombat.BP_MasterCombat_C|GetEnemyToFight _asbp_master_combat))))) (Math|Float|Square 3e+03))))))) (* -9.8e+02 (Math|Vector2D|Vector2DLength (- (Math|Vector2D|MakeVector2D (.X (Math|Vector|BreakVector (Transformation|GetActorLocation (Variables|/Game/MasterBlueprints/Units/BP_MasterCombat.BP_MasterCombat_C|GetEnemyToFight _asbp_master_combat)))) (.Y (Math|Vector|BreakVector (Transformation|GetActorLocation (Variables|/Game/MasterBlueprints/Units/BP_MasterCombat.BP_MasterCombat_C|GetEnemyToFight _asbp_master_combat))))) (Math|Vector2D|MakeVector2D (.X (Math|Vector|BreakVector (Transformation|GetActorLocation _asbp_master_combat))) (.Y (Math|Vector|BreakVector (Transformation|GetActorLocation _asbp_master_combat))))))))) _returnvalue_3) (+ (.yaw _returnvalue_5) _returnvalue_3)) false false)))
        (Game|SpawnActorfromClass "/Game/Blueprints/Items/Projectiles/BP_BasicRifleBullet.BP_BasicRifleBullet_C" (Math|Transform|MakeTransform (.location _returnvalue_4) (.rotation _returnvalue_4) "1,1,1") "Undefined" 0 _weaponowner_2 (Variables|Default|GetWeaponDamage) 0)
        (Utilities|Time|SetTimerbyFunctionName 0 "Fire" (Math|Random|RandomFloatinRange 0.2 0.5))))))