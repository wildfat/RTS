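; BP_BasicAxe is an axe weapon that damages actors through hit box overlaps.
; HitBox overlaps call ApplyDamageToHitActor, which requires CanDamage, skips the owner and accepts only box components whose first tag is "HitBox".
; It records victims in DamagedActors to prevent repeat hits, then applies WeaponDamage with the owner as causer.
; An owner-versus-victim tag comparison exists, but both branches are empty, so it filters nothing.
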(event OnComponentBeginOverlap(HitBox)
  (params (OverlappedComponent :type Primitive%20Component%20Object%20Reference) (OtherActor :type Actor%20Object%20Reference) (OtherComp :type Primitive%20Component%20Object%20Reference) (OtherBodyIndex :type Integer) (bFromSweep :type Boolean) (SweepResult :type Hit%20Result%20Structure%20%28by%20ref%29))
  (CallFunction|ApplyDamagetoHitActor OtherActor OtherComp))

(event EventBeginPlay
  (|CallParentFunction) ; This node is disabled and will not be called.\nDrag off pins to build functionality.
)

(event Collision|EventActorBeginOverlap
  (params (OtherActor :type Actor%20Object%20Reference))
  (|CallParentFunction OtherActor) ; This node is disabled and will not be called.\nDrag off pins to build functionality.
)

(event EventTick
  (params (DeltaSeconds :type Float%20%28single-precision%29))
  (|CallParentFunction DeltaSeconds) ; This node is disabled and will not be called.\nDrag off pins to build functionality.
)

(fn ConstructionScript
  (|CallParentFunction))

(fn ApplyDamagetoHitActor
  (params (InHitActor :type Actor%20Object%20Reference) (InHitBox :type Object%20Object%20Reference))
  (bind _weaponowner (Variables|Default|GetWeaponOwner))
  (bind _damagedactors (Variables|Default|GetDamagedActors))
  (if (Variables|Default|GetCanDamage)
    (if (== InHitActor _weaponowner)
      _
      (else
        (bind _asbox_collision (Utilities|Casting|CastToBoxComponent InHitBox)
          (:then
            (if (Utilities|Name|Equal(Name) (Utilities|Array|Get(acopy) (Variables|/Script/Engine.ActorComponent|GetComponentTags _asbox_collision)) "HitBox")
              (if (Utilities|Name|Equal(Name) (Utilities|Array|Get(acopy) (Variables|/Script/Engine.Actor|GetTags (Components|GetOwner _asbox_collision))) (Utilities|Array|Get(acopy) (Variables|/Script/Engine.Actor|GetTags _weaponowner)))
                _
                (else
                  _))
              (if (Utilities|Array|ContainsItem _damagedactors (Components|GetOwner _asbox_collision))
                _
                (else
                  (Utilities|Array|Add _damagedactors (Components|GetOwner _asbox_collision))
                  (Game|Damage|ApplyDamage (Components|GetOwner _asbox_collision) (Variables|Default|GetWeaponDamage) 0 (Variables|Default|GetWeaponOwner))))))
          (:CastFailed
            _)))))
  (return 0))