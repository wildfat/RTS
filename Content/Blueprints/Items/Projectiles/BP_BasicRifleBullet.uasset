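; Rifle bullet projectile that damages the actor it hits, with its logic in ApplyDamageToHitActor and an empty event graph.
; With a valid shooter, only box components whose second tag is BodyHitBox take damage, and BP_MasterUnit TeamName comparison blocks friendly fire.
; Without a valid shooter, damage skips those checks.
; Impacts then spawn a pooled particle effect using the shooter's yaw and destroy the bullet.
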(event EventBeginPlay
  (|CallParentFunction) ; This node is disabled and will not be called.\nDrag off pins to build functionality.
)

(event Collision|EventActorBeginOverlap
  (params (OtherActor :type Actor%20Object%20Reference)))

(event EventTick
  (params (DeltaSeconds :type Float%20%28single-precision%29)))

(fn ConstructionScript
  (|CallParentFunction))

(fn ApplyDamagetoHitActor
  (params (InHitBox :type Object%20Object%20Reference) (InHitActor :type Actor%20Object%20Reference) (InHitLocation :type Vector :default "0, 0, 0"))
  (bind _firedfrom (Variables|Default|GetFiredFrom))
  (Utilities|IsValid (Variables|Default|GetFiredFrom)
    (:Is%20Valid
      (Utilities|IsValid InHitActor
        (:Is%20Valid
          (bind _asbox_collision (Utilities|Casting|CastToBoxComponent InHitBox)
            (:then
              ;[1 1 1] HeadshotExmpl
              (if (Utilities|Name|Equal(Name) (Utilities|Array|Get(acopy) (Variables|/Script/Engine.ActorComponent|GetComponentTags _asbox_collision) 1) "BodyHitBox")
                (Variables|Default|SetProjectileDamage (* (Variables|Default|GetProjectileDamage) 1.0))
                (if (Utilities|Name|Equal(Name) (Variables|/Game/MasterBlueprints/Units/BP_MasterUnit.BP_MasterUnit_C|GetTeamName (.AsBP%20Master%20Unit (Utilities|Casting|CastToBP_MasterUnit (Components|GetOwner _asbox_collision)))) (Variables|/Game/MasterBlueprints/Units/BP_MasterUnit.BP_MasterUnit_C|GetTeamName (.AsBP%20Master%20Unit (Utilities|Casting|CastToBP_MasterUnit (Variables|Default|GetFiredFrom)))))
                  _
                  (else
                    (Game|Damage|ApplyDamage InHitActor (Variables|Default|GetProjectileDamage) 0 _firedfrom)))))
            (:CastFailed
              _)))
        (:Is%20Not%20Valid
          _))
      (Utilities|IsValid _firedfrom
        (:Is%20Valid
          _)))
    (:Is%20Not%20Valid
      (Game|Damage|ApplyDamage InHitActor (Variables|Default|GetProjectileDamage) 0 0)))
  (Effects|SpawnEmitteratLocation (Variables|Default|GetImpactParticleEffect) InHitLocation (Math|Rotator|MakeRotator 0.0 0.0 (.yaw (Transformation|GetActorRotation _firedfrom))) "1.000000,1.000000,1.000000" true "AutoRelease")
  (Actor|DestroyActor)
  (return 0))