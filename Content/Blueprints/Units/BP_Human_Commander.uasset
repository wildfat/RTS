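; BP_Human_Commander is the human commander unit, a child Blueprint that supplies the human-specific HUD and building list.
; On BeginPlay it runs StartUp and prints a debug "Hello" when locally controlled or running on the server.
; CreateWidgets extends the parent's version, adding W_HumanCommanderHUD to the viewport with gold text and a commander reference, then handing it a newly created W_Human_BuildingList.
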(event EventBeginPlay
  (if (Pawn|IsLocallyControlled)
    (CallFunction|StartUp :!label _label)
    (Development|PrintString "Hello")
    (elif (Networking|IsServer)
      (goto _label))))

(fn ConstructionScript
  (|CallParentFunction))

(fn CreateWidgets
  (bind _return (|CallParentFunction))
  (bind _returnvalue (UserInterface|CreateWidget "/Game/Widgets/HumanWidgets/W_HumanCommanderHUD.W_HumanCommanderHUD_C" 0 (Utilities|Text|ToText(Float) (Variables|Default|GetGold) "HalfToEven" false true 1 324 0 0) self))
  (bind _output_get (Variables|Default|SetCommanderHud _returnvalue))
  (UserInterface|Viewport|AddtoViewport _output_get 0)
  (bind _returnvalue_2 (UserInterface|CreateWidget "/Game/Widgets/HumanWidgets/Lists/W_Human_BuildingList.W_Human_BuildingList_C" 0 self))
  (Variables|Default|SetBuilfingListWidget _returnvalue_2)
  (bind _asw_human_commander_hud (Utilities|Casting|CastToW_HumanCommanderHUD (Variables|Default|GetCommanderHud))
    (:then
      (Variables|/Game/Widgets/HumanWidgets/W_HumanCommanderHUD.W_HumanCommanderHUD_C|SetBuildingList _asw_human_commander_hud (Variables|Default|GetBuilfingListWidget)))
    (:CastFailed
      _))
  (return _return))