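; Human barracks building for the RTS commander, a child building class that provides the infantry unit list.
; It creates its own infantry list widget, bound to the local commander and itself as builder.
; The first locally controlled barrack with a matching tag registers its list as the HUD default and enables infantry.
; Selecting a finished local barrack shows its own list on the commander HUD; deselecting restores the default list.
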(event EventBeginPlay
  (CallFunction|StartUp))

(fn ConstructionScript
  (|CallParentFunction)
  (Variables|Default|SetMaxHealth 1e+03)
  (Variables|Default|SetHealthFillSpeed 3.0)
  (Variables|Default|SetListName "InfantryList"))

(fn CreateWidgets
  (bind _return (|CallParentFunction))
  (bind _returnvalue (UserInterface|CreateWidget "/Game/Widgets/HumanWidgets/Lists/W_Human_InfantryList.W_Human_InfantryList_C" 0 (Variables|Default|GetLocalCommander) self))
  (Variables|Default|SetUnitListWidget _returnvalue)
  (return _return))

(fn CheckFirstOfItsKind
  (bind _localcommander (Variables|Default|GetLocalCommander))
  (bind _return (|CallParentFunction))
  (Utilities|IsValid _localcommander
    (:Is%20Valid
      (if (Pawn|IsLocallyControlled _localcommander)
        (bind _outactors (Actor|GetAllActorsOfClass "BP_HumanBarrack_C"))
        (for _array_element _outactors
          (if (Pawn|IsLocallyControlled (Variables|/Game/MasterBlueprints/Units/BP_MasterBuilding.BP_MasterBuilding_C|GetLocalCommander _array_element))
            (if (Utilities|Name|Equal(Name) (Utilities|Array|Get(acopy) (Variables|/Script/Engine.Actor|GetTags _array_element)) (Utilities|Array|Get(acopy) (Variables|Default|GetTags)))
              (Variables|Default|SetNumberOfSimilarBuilding (+ (Variables|Default|GetNumberOfSimilarBuilding) 1)))))
        (if (== (Variables|Default|GetNumberOfSimilarBuilding) 1)
          (bind _asw_human_commander_hud (Utilities|Casting|CastToW_HumanCommanderHUD (Variables|Default|GetCommanderHud))
            (:then
              (bind _output_get (Variables|/Game/Widgets/HumanWidgets/W_HumanCommanderHUD.W_HumanCommanderHUD_C|SetDefaultInfantryList _asw_human_commander_hud (Variables|Default|GetUnitListWidget)))
              (Variables|/Game/Widgets/HumanWidgets/W_HumanCommanderHUD.W_HumanCommanderHUD_C|SetInfantryList _asw_human_commander_hud _output_get)
              (Variables|/Game/Widgets/HumanWidgets/W_HumanCommanderHUD.W_HumanCommanderHUD_C|SetInfantryListEnable _asw_human_commander_hud true))
            (:CastFailed
              _)))))
    (:Is%20Not%20Valid
      _))
  (return _return))

(fn WhenImSelected
  (bind (_finishedbuilding _commanderislocal) (|CallParentFunction))
  (if _finishedbuilding
    (if _commanderislocal
      (bind _asw_human_commander_hud (Utilities|Casting|CastToW_HumanCommanderHUD (Variables|Default|GetCommanderHud))
        (:then
          (Variables|/Game/Widgets/HumanWidgets/W_HumanCommanderHUD.W_HumanCommanderHUD_C|SetInfantryList _asw_human_commander_hud (Variables|Default|GetUnitListWidget))
          (Default|ShowDesiredList _asw_human_commander_hud (Variables|Default|GetListName)))
        (:CastFailed
          _))))
  (return _finishedbuilding _commanderislocal))

(fn WhenImNotSelected
  (bind _return (|CallParentFunction))
  (bind _asw_human_commander_hud (Utilities|Casting|CastToW_HumanCommanderHUD (Variables|Default|GetCommanderHud))
    (:then
      (Variables|/Game/Widgets/HumanWidgets/W_HumanCommanderHUD.W_HumanCommanderHUD_C|SetInfantryList _asw_human_commander_hud (Variables|/Game/Widgets/HumanWidgets/W_HumanCommanderHUD.W_HumanCommanderHUD_C|GetDefaultInfantryList _asw_human_commander_hud))
      (Default|ShowDesiredList _asw_human_commander_hud (Variables|Default|GetListName)))
    (:CastFailed
      _))
  (return _return))