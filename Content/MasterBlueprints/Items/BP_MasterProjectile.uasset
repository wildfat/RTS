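; Master projectile Blueprint, a base for projectiles fired from weapons.
; On BeginPlay, StartUp adds weapon damage to projectile damage, sets the lifespan, and calls IgnoreActorWhenMoving on the firing actor with ShouldIgnore off, so the shooter is not ignored.
; Hit events pass the struck component, actor and location to ApplyDamageToHitActor, which is a stub here that only returns zero and applies no damage.
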(event EventBeginPlay
  (CallFunction|StartUp))

(event Collision|EventHit
  (params (MyComp :type Primitive%20Component%20Object%20Reference) (Other :type Actor%20Object%20Reference) (OtherComp :type Primitive%20Component%20Object%20Reference) (bSelfMoved :type Boolean) (HitLocation :type Vector :default "0, 0, 0") (HitNormal :type Vector :default "0, 0, 0") (NormalImpulse :type Vector :default "0, 0, 0") (Hit :type Hit%20Result%20Structure%20%28by%20ref%29))
  (CallFunction|ApplyDamagetoHitActor OtherComp Other HitLocation))

(fn ConstructionScript)

(fn StartUp
  (Variables|Default|SetProjectileDamage (+ (Variables|Default|GetProjectileDamage) (Variables|Default|GetWeaponDamage)))
  (Collision|IgnoreActorwhenMoving (Variables|Default|GetProjectileCollision) (Variables|Default|GetFiredFrom) false)
  (Actor|SetLifeSpan (Variables|Default|GetProjectileLifeSpan)))

(fn ApplyDamagetoHitActor
  (params (InHitBox :type Object%20Object%20Reference) (InHitActor :type Actor%20Object%20Reference) (InHitLocation :type Vector))
  (return 0))