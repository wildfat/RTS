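; BP_MasterMelee is a base Blueprint for melee items, holding shared damage-window state and a hit function.
; SetDamageEnable stores the CanDamage flag and clears the DamagedActors list when damage is switched off.
; ApplyDamageToHitActor takes a hit actor and hit box but only returns zero, applying no damage here.
; The event graph holds only disabled default events, and construction just calls the parent.
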(event EventBeginPlay
  (|CallParentFunction) ; This node is disabled and will not be called.\nDrag off pins to build functionality.
)

(event Collision|EventActorBeginOverlap
  (params (OtherActor :type Actor%20Object%20Reference))
  (|CallParentFunction OtherActor) ; This node is disabled and will not be called.\nDrag off pins to build functionality.
)

(event EventTick
  (params (DeltaSeconds :type Float%20%28single-precision%29))
  (|CallParentFunction DeltaSeconds) ; This node is disabled and will not be called.\nDrag off pins to build functionality.
)

(fn ConstructionScript
  (|CallParentFunction))

(fn SetDamageEnable
  (params (CanDamage :type Boolean))
  (bind _output_get (Variables|Default|SetCanDamage CanDamage))
  (if (not _output_get)
    (Utilities|Array|Clear (Variables|Default|GetDamagedActors))))

(fn ApplyDamagetoHitActor
  (params (InHitActor :type Actor%20Object%20Reference) (InHitBox :type Object%20Object%20Reference))
  (return 0))