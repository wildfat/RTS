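; Master base for unit-producing buildings, extending a parent selectable building with a spawn point and a rally-style spawn flag.
; Selection activates the flag only when construction is finished and the commander is local; deselection deactivates it.
; Spawn requests go to the local commander's ROSSpawnUnit with the spawn point transform and flag location.
; When the parent's health fill reports completion, it calls CheckFirstOfItsKind, an empty stub here.
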(event EventImSelected
  (CallFunction|WhenImSelected))

(fn ConstructionScript
  (|CallParentFunction))

(fn WhenImSelected
  (bind (_finishedbuilding _commanderislocal) (|CallParentFunction))
  (if _finishedbuilding
    (if _commanderislocal
      (Components|Activation|Activate (Variables|Default|GetSpawnFlag) false)))
  (return _finishedbuilding _commanderislocal))

(fn WhenImNotSelected
  (bind _return (|CallParentFunction))
  (Components|Activation|Deactivate (Variables|Default|GetSpawnFlag))
  (return _return))

(fn ToCommanderSpawnUnit
  (params (InUnit :type BP%20Master%20Unit%20Class%20Reference))
  (bind _asbp_dss_master_commander (Utilities|Casting|CastToBP_DSS_MasterCommander (Variables|Default|GetLocalCommander)))
  (Default|ROSSpawnUnit _asbp_dss_master_commander InUnit (Transformation|GetWorldTransform (Variables|Default|GetSpawnPoint)) _asbp_dss_master_commander (Transformation|GetWorldLocation (Variables|Default|GetSpawnFlag))))

(fn CheckFirstOfItsKind
  (return 0))

(fn HealthFillComleted
  (bind _finishedbuilding (|CallParentFunction))
  (if _finishedbuilding
    (CallFunction|CheckFirstOfItsKind))
  (return _finishedbuilding))