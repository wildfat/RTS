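; Base RTS building Blueprint that handles the construction phase, health bar and selection response.
; StartUp caches commander, HUD and team tag from the game instance, then a looping timer fills health while raising the mesh from UnderFloor to OnFloor in proportion.
; At full health it marks construction finished and hides the bar.
; A second timer rotates the bar toward the commander camera during construction or selection; CreateWidgets is an empty stub.
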(event EventImSelected
  (Utilities|Time|SetTimerbyFunctionName 0 "HealthBarFollowsCamera" 0.01 true)
  (Utilities|FlowControl|Delay 0.1)
  (CallFunction|WhenImSelected self))

(event EventImNotSelected
  (Utilities|Time|ClearTimerbyFunctionName 0 "HealthBarFollowsCamera")
  (Utilities|FlowControl|Delay 0.1)
  (CallFunction|WhenImNotSelected self))

(fn ConstructionScript)

(fn WhenImSelected
  (bind _finishedbuilding (Variables|Default|GetFinishedBuilding))
  (bind _localcommander (Variables|Default|GetLocalCommander))
  (bind _returnvalue (Pawn|IsLocallyControlled _localcommander))
  (if _finishedbuilding
    (Rendering|SetVisibility (Variables|Default|GetHealthBar) true false)
    (Utilities|IsValid _localcommander
      (:Is%20Valid
        (if _returnvalue
          _
          (else
            _)))))
  (return _finishedbuilding _returnvalue))

(fn WhenImNotSelected
  (Rendering|SetVisibility (Variables|Default|GetHealthBar) false false)
  (return 0))

(fn StartUp
  (Variables|Default|SetFinishedBuilding false)
  (CallFunction|SerGameInstanceVariable)
  (Transformation|SetWorldLocation (Variables|Default|GetBuildingMesh) (Transformation|GetWorldLocation (Variables|Default|GetUnderFloor)) false false)
  (Rendering|SetVisibility (Variables|Default|GetHealthBar) true false)
  (Utilities|Time|SetTimerbyFunctionName 0 "HealthBarFollowsCamera" 0.01 true)
  (CallFunction|CreateWidgets)
  (CallFunction|StartHealthFill)
  (return 0))

(fn StartHealthFill
  (Utilities|Time|SetTimerbyFunctionName 0 "HealthFill" 0.01 true))

(fn StopHealthFill
  (Utilities|Time|ClearTimerbyFunctionName 0 "HealthFill"))

(fn HealthFill
  (bind _buildingmesh (Variables|Default|GetBuildingMesh))
  (bind _underfloor (Variables|Default|GetUnderFloor))
  (bind _maxhealth (Variables|Default|GetMaxHealth))
  (bind _returnvalue (Transformation|GetWorldLocation _buildingmesh))
  (bind _returnvalue_2 (Transformation|GetWorldLocation _underfloor))
  (bind _output_get (Variables|Default|SetCurrentHealth (Math|Float|Clamp(Float) (+ (Variables|Default|GetCurrentHealth) (Variables|Default|GetHealthFillSpeed)) 0.0 _maxhealth)))
  (bind _asw_health_bar (Utilities|Casting|CastToW_HealthBar (UserInterface|GetUserWidgetObject (Variables|Default|GetHealthBar))))
  (Variables|/Game/Widgets/W_HealthBar.W_HealthBar_C|SetHealthPercent _asw_health_bar (/ _output_get _maxhealth))
  (Transformation|SetWorldLocation _buildingmesh (Math|Vector|MakeVector (.x _returnvalue) (.y _returnvalue) (+ (* (/ _output_get _maxhealth) (- (.z (Transformation|GetWorldLocation (Variables|Default|GetOnFloor))) (.z _returnvalue_2))) (.z _returnvalue_2))) false false)
  (if (== (/ _output_get _maxhealth) 1.0)
    (CallFunction|HealthFillComleted)))

(fn HealthFillComleted
  (CallFunction|StopHealthFill)
  (Utilities|Time|ClearTimerbyFunctionName 0 "HealthBarFollowsCamera")
  (Transformation|SetWorldLocation (Variables|Default|GetBuildingMesh) (Transformation|GetWorldLocation (Variables|Default|GetOnFloor)) false false)
  (Rendering|SetVisibility (Variables|Default|GetHealthBar) false false)
  (bind _output_get (Variables|Default|SetFinishedBuilding true))
  (return _output_get))

(fn HealthBarFollowsCamera
  (bind _healthbar (Variables|Default|GetHealthBar))
  (bind _asbp_dss_master_commander (Utilities|Casting|CastToBP_DSS_MasterCommander (Variables|Default|GetAllCommander)))
  (Transformation|SetWorldRotation _healthbar (Math|Rotator|MakeRotator (+ 9e+01 (.pitch (Transformation|GetWorldRotation (Variables|/Game/MasterBlueprints/Units/BP_DSS_MasterCommander.BP_DSS_MasterCommander_C|GetCamera _asbp_dss_master_commander)))) (.pitch (Transformation|GetWorldRotation _healthbar)) (+ (.yaw (Transformation|GetWorldRotation (Variables|/Game/MasterBlueprints/Units/BP_DSS_MasterCommander.BP_DSS_MasterCommander_C|GetCamera _asbp_dss_master_commander))) 9e+01)) false false))

(fn SerGameInstanceVariable
  (bind _asdss_game_instance (Utilities|Casting|CastToDSS_GameInstance (Game|GetGameInstance)))
  (Variables|Default|SetAllCommander (Variables|/Game/Blueprints/Logics/DSS_GameInstance.DSS_GameInstance_C|GetCommander _asdss_game_instance))
  (Variables|Default|SetCommanderHud (Variables|/Game/Blueprints/Logics/DSS_GameInstance.DSS_GameInstance_C|GetCommanderHud _asdss_game_instance))
  (Utilities|Array|SetArrayElem (Variables|Actor|GetTags) 0 (Variables|/Game/Blueprints/Logics/DSS_GameInstance.DSS_GameInstance_C|GetTeamName _asdss_game_instance)))

(fn CreateWidgets
  (return 0))