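; Base infantry unit for a commander-controlled strategy game, with selection visuals, health, death and move orders that override its AI.
; It spawns two weapons; equipping one sets the fighting style, behavior tree and blackboard ranges.
; Sightings, damage or distress calls set the blackboard enemy and InCombat, whose RepNotify runs timers for facing and camera-aligned health bar.
; Attacks branch by fighting style into multicast montages with timed axe damage or rifle fire.
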(event Custom|ROS_SpawnInitialWeapons
  (Utilities|FlowControl|Delay 0.01)
  (Weapon|SpawnInitialWeapons))

(event Custom|AttackEnemy
  (Utilities|CheckFightingStyle))

(event Custom|MC_PlayMontage
  (params (InAnimMontage :type Anim%20Montage%20Object%20Reference))
  (bind _returnvalue (Animation|PlayAnimMontage InAnimMontage 1.0 "None"))
  (Variables|Default|SetAnimDelay _returnvalue))

(event Custom|ROS_StopMontage
  (CallFunction|MCStopMontage))

(event Custom|MC_StopMontage
  (bind _returnvalue (Animation|GetCurrentMontage :!class /Script/Engine.Character))
  (Animation|StopAnimMontage _returnvalue))

(event EventBeginPlay
  (CallFunction|StartUp))

(event Game|Damage|EventAnyDamage
  (params (Damage :type Float%20%28single-precision%29) (DamageType :type Damage%20Type%20Object%20Reference) (InstigatedBy :type Controller%20Object%20Reference) (DamageCauser :type Actor%20Object%20Reference))
  (CallFunction|OnDamaged Damage DamageCauser))

(event EventMovebyCommander
  (params (InLocation :type Vector :default "0, 0, 0"))
  (Utilities|FlowControl|Delay 0.1)
  (CallFunction|MovetobyCommander InLocation))

(fn ConstructionScript
  (|CallParentFunction))

(fn WhenImSelected
  (bind _localcommander (Variables|Default|GetLocalCommander))
  (bind _returnvalue (Pawn|IsLocallyControlled _localcommander))
  (Rendering|SetVisibility (Variables|Default|GetSelectionDecal) true false)
  (if (Variables|Combat|GetInCombat)
    _
    (else
      (Utilities|Time|SetTimerbyFunctionName 0 "HealthBarFollowsCamera" 0.01 true)
      (Rendering|SetVisibility (Variables|Default|GetHealthBar) true false)))
  (Variables|Default|SetImSelectedBool true)
  (Utilities|IsValid _localcommander
    (:Is%20Valid
      (if _returnvalue
        _
        (else
          _)))
    (:Is%20Not%20Valid
      _))
  (return _returnvalue))

(fn WhenImNotSelected
  (Rendering|SetVisibility (Variables|Default|GetSelectionDecal) false false)
  (if (Variables|Combat|GetInCombat)
    _
    (else
      (Utilities|Time|ClearTimerbyFunctionName 0 "HealthBarFollowsCamera")
      (Rendering|SetVisibility (Variables|Default|GetHealthBar) false false)))
  (Variables|Default|SetImSelectedBool false)
  (return 0))

(fn OnSeeEnemies
  (params (InEnemy :type Actor%20Object%20Reference))
  (bind _returnvalue (AI|GetBlackboard 0))
  (Utilities|IsValid _returnvalue
    (:Is%20Valid
      (AI|Components|Blackboard|SetValueasObject _returnvalue (Variables|Default|GetBBK_EnemyToFight) InEnemy)
      (Variables|Default|SetEnemyToFight InEnemy)
      (Variables|Combat|SetInCombat true)
      (AI|Components|Blackboard|SetValueasBool _returnvalue (Variables|Default|GetBBK_EnemyVisible) true)
      (Utilities|Time|SetTimerbyFunctionName 0 "UnitedWeStand" 0.5)
      (return 0))))

(fn OnDamaged
  (params (InDamage :type Float%20%28single-precision%29) (InDamageCauser :type Actor%20Object%20Reference))
  (bind _output_get (Variables|Default|SetCurrentHealth (Math|Float|Clamp(Float) (- (Variables|Default|GetCurrentHealth) InDamage) 0.0 (Variables|Default|GetMaxHealth))))
  (if (== _output_get 0.0)
    (CallFunction|OnDeath)
    (else
      (Utilities|IsValid (Variables|Default|GetEnemyToFight)
        (:Is%20Valid
          _)
        (:Is%20Not%20Valid
          (Utilities|IsValid InDamageCauser
            (:Is%20Valid
              (CallFunction|OnSeeEnemies InDamageCauser))
            (:Is%20Not%20Valid
              _))))))
  (return 0))

(fn Disengage
  (bind _returnvalue (AI|GetBlackboard 0))
  (bind _returnvalue_2 (Utilities|Name|MakeLiteralName "EnemyToFight"))
  (Utilities|IsValid _returnvalue
    (:Is%20Valid
      (AI|Components|Blackboard|SetValueasObject _returnvalue _returnvalue_2 0)
      (Variables|Default|SetEnemyToFight 0)
      (Variables|Combat|SetInCombat false)
      (AI|Components|Blackboard|SetValueasBool _returnvalue _returnvalue_2 false)
      (return 0))))

(fn OnDeath
  (for _array_element (Variables|Weapon|GetWeapons)
    (Utilities|IsValid _array_element
      (:Is%20Valid
        (Actor|DestroyActor _array_element))))
  (Actor|DestroyActor)
  (return 0))

(fn OnRepinCombat
  (bind _healthbar (Variables|Default|GetHealthBar))
  (if (Variables|Combat|GetInCombat)
    (Rendering|SetVisibility _healthbar true false)
    (if (not (Class|KismetSystemLibrary|TimerExists 0 "LookAtEnemy"))
      (Utilities|Time|SetTimerbyFunctionName 0 "LookAtEnemy" 0.01 true))
    (else
      (Utilities|Time|ClearTimerbyFunctionName 0 "LookAtEnemy")
      (if (Variables|Default|GetImSelectedBool)
        (Utilities|Time|SetTimerbyFunctionName 0 "HealthBarFollowsCamera" 0.01 true)
        (else
          (Rendering|SetVisibility _healthbar false false))))))

(fn MovetoLocation
  (params (InLocation :type Vector :default "0, 0, 0"))
  (CallFunction|ROSStopMontage)
  (Class|DSSInterface|Moveto(Message) (Pawn|GetController) InLocation)
  (return 0))

(fn SpawnInitialWeapons
  (bind _returnvalue (Transformation|GetActorTransform))
  (bind _returnvalue_2 (Game|SpawnActorfromClass (Variables|Weapon|GetPrimaryWeaponClass) _returnvalue "Undefined" 0 self 0))
  (Utilities|Array|SetArrayElem (Variables|Weapon|GetWeapons) 0 _returnvalue_2 true)
  (Variables|Weapon|SetWeaponInHand _returnvalue_2)
  (bind _returnvalue_3 (Game|SpawnActorfromClass (Variables|Weapon|GetSecondaryWeaponClass) _returnvalue "Undefined" 0 self 0))
  (Utilities|Array|SetArrayElem (Variables|Weapon|GetWeapons) 1 _returnvalue_3 true)
  (Weapon|EquipWeapon)
  (for (_array_element _array_index) (Variables|Weapon|GetWeapons)
    (if (> _array_index 0)
      (bind _asbp_master_weapon (Utilities|Casting|CastToBP_MasterWeapon _array_element))
      (Transformation|AttachComponentToComponent _asbp_master_weapon (Variables|Character|GetMesh) (Variables|/Game/MasterBlueprints/Items/BP_MasterWeapon.BP_MasterWeapon_C|GetAttachOffHandSocket _asbp_master_weapon) "SnapToTarget" "SnapToTarget" "SnapToTarget" true))))

(fn EquipWeapon
  (params (InWeaponIndexNumber :type Integer))
  (bind _asbp_master_weapon (Utilities|Casting|CastToBP_MasterWeapon (Variables|Weapon|GetWeaponInHand)))
  (Transformation|AttachComponentToComponent _asbp_master_weapon (Variables|Character|GetMesh) (Variables|/Game/MasterBlueprints/Items/BP_MasterWeapon.BP_MasterWeapon_C|GetAttachOffHandSocket _asbp_master_weapon) "SnapToTarget" "SnapToTarget" "SnapToTarget" true)
  (bind _output_get (Variables|Weapon|SetWeaponInHand (Utilities|Array|Get(acopy) (Variables|Weapon|GetWeapons) InWeaponIndexNumber)))
  (bind _asbp_master_weapon_2 (Utilities|Casting|CastToBP_MasterWeapon _output_get))
  (Variables|Combat|SetFightingStyle (Variables|/Game/MasterBlueprints/Items/BP_MasterWeapon.BP_MasterWeapon_C|GetFightingStyle _asbp_master_weapon_2))
  (Transformation|AttachComponentToComponent _asbp_master_weapon_2 (Variables|Character|GetMesh) (Variables|/Game/MasterBlueprints/Items/BP_MasterWeapon.BP_MasterWeapon_C|GetAttachInHandSocket _asbp_master_weapon_2) "SnapToTarget" "SnapToTarget" "SnapToTarget" true)
  (Class|DSSInterface|SwitchBehaviorTree(Message) (Pawn|GetController) (Variables|/Game/MasterBlueprints/Items/BP_MasterWeapon.BP_MasterWeapon_C|GetBehaviorTree _asbp_master_weapon_2))
  (AI|Components|Blackboard|SetValueasFloat (AI|GetBlackboard 0) (Variables|BBK|GetBBK_WeaponRange) (Variables|/Game/MasterBlueprints/Items/BP_MasterWeapon.BP_MasterWeapon_C|GetWeaponRange _asbp_master_weapon_2))
  (AI|Components|Blackboard|SetValueasFloat (AI|GetBlackboard 0) (Variables|Default|GetBBK_DisengagePreFightRange) (Variables|Default|GetDisengagePreFightRange))
  (AI|Components|Blackboard|SetValueasFloat (AI|GetBlackboard 0) (Variables|Default|GetBBK_DisengageEnemyRange) (Variables|Default|GetDisengageEnemyRange)))

(fn StartUp
  (bind _return (|CallParentFunction))
  (CallFunction|ROSSpawnInitialWeapons)
  (return _return))

(fn MovetobyCommander
  (params (InLocation :type Vector))
  (bind _returnvalue (AI|GetBlackboard 0))
  (Utilities|IsValid _returnvalue
    (:Is%20Valid
      (AI|Components|Blackboard|SetValueasVector _returnvalue (Variables|Default|GetBBK_Test) InLocation)
      (bind _output_get (Variables|Default|SetOverrideAllOtherActions true))
      (AI|Components|Blackboard|SetValueasBool _returnvalue (Variables|Default|GetBBK_OverrideAllOtherActions) _output_get)
      (CallFunction|MovetoLocation InLocation))))

(fn LookatEnemy
  (bind _returnvalue (Transformation|GetActorRotation))
  (bind _healthbar (Variables|Default|GetHealthBar))
  (Utilities|FlowControl|Sequence
    (:then_0
      (if (not (Variables|Default|GetOverrideAllOtherActions))
        (Utilities|IsValid (Variables|Default|GetEnemyToFight)
          (:Is%20Valid
            (Transformation|SetActorRotation (Math|Rotator|MakeRotator (.roll _returnvalue) (.pitch _returnvalue) (.yaw (Math|Rotator|FindLookatRotation (Transformation|GetActorLocation) (Transformation|GetActorLocation (Variables|Default|GetEnemyToFight)))))))
          (:Is%20Not%20Valid
            (CallFunction|Disengage)))))
    (:then_1
      (bind _asbp_dss_master_commander (Utilities|Casting|CastToBP_DSS_MasterCommander (Variables|Default|GetAllCommander)))
      (Transformation|SetWorldRotation _healthbar (Math|Rotator|MakeRotator (+ 9e+01 (.pitch (Transformation|GetWorldRotation (Variables|/Game/MasterBlueprints/Units/BP_DSS_MasterCommander.BP_DSS_MasterCommander_C|GetCamera _asbp_dss_master_commander)))) (.pitch (Transformation|GetWorldRotation _healthbar)) (+ (.yaw (Transformation|GetWorldRotation (Variables|/Game/MasterBlueprints/Units/BP_DSS_MasterCommander.BP_DSS_MasterCommander_C|GetCamera _asbp_dss_master_commander))) 9e+01)) false false))))

(fn DistressCall
  (params (InEnemy :type Actor%20Object%20Reference))
  (Utilities|IsValid InEnemy
    (:Is%20Valid
      (Utilities|IsValid (Variables|Default|GetEnemyToFight)
        (:Is%20Valid
          _)
        (:Is%20Not%20Valid
          (CallFunction|OnSeeEnemies InEnemy))))
    (:Is%20Not%20Valid
      _))
  (return 0))

(fn OnBumpbyFriendly
  (params (InBoxCollision :type Object%20Object%20Reference) (InActor :type Actor%20Object%20Reference))
  (return))