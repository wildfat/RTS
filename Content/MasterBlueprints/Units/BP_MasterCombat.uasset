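; BP_MasterCombat is a base Blueprint for team-based combat units, with empty sighting, damage, disengage, death and distress-call functions.
; A danger box treats opposing combat units or projectile shooters as sighted enemies while no target is valid.
; UnitedWeStand sphere-traces nearby and passes the current enemy to the first same-team hit via DistressCall.
; Friendly capsule bumps set a blackboard move flag, clearing the action override if fighting.
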(event OnComponentBeginOverlap(DangerDetectionBox)
  (params (OverlappedComponent :type Primitive%20Component%20Object%20Reference) (OtherActor :type Actor%20Object%20Reference) (OtherComp :type Primitive%20Component%20Object%20Reference) (OtherBodyIndex :type Integer) (bFromSweep :type Boolean) (SweepResult :type Hit%20Result%20Structure%20%28by%20ref%29))
  (Combat|OnDangerDetected OtherActor))

(event OnComponentBeginOverlap(BumpBox)
  (params (OverlappedComponent :type Primitive%20Component%20Object%20Reference) (OtherActor :type Actor%20Object%20Reference) (OtherComp :type Primitive%20Component%20Object%20Reference) (OtherBodyIndex :type Integer) (bFromSweep :type Boolean) (SweepResult :type Hit%20Result%20Structure%20%28by%20ref%29))
  (Combat|OnBumpbyFriendly OtherComp OtherActor))

(fn ConstructionScript
  (|CallParentFunction))

(fn OnSeeEnemies
  (params (InEnemy :type Actor%20Object%20Reference))
  (return 0))

(fn OnDamaged
  (params (InDamage :type Float%20%28single-precision%29) (InDamageCauser :type Actor%20Object%20Reference))
  (return 0))

(fn Disengage
  (return 0))

(fn OnDeath
  (return 0))

(fn UnitedWeStand
  (bind _returnvalue (Transformation|GetActorLocation))
  (bind _outhits (Collision|MultiSphereTraceForObjects _returnvalue (+ _returnvalue "0, 0, 0") 2e+03 (Utilities|Array|MakeArray "ObjectTypeQuery2" "ObjectTypeQuery3") false 0 "None"))
  (for _array_element _outhits
    (if (Utilities|Name|Equal(Name) (Variables|/Game/MasterBlueprints/Units/BP_MasterUnit.BP_MasterUnit_C|GetTeamName (.AsBP%20Master%20Unit (Utilities|Casting|CastToBP_MasterUnit (.HitActor (Collision|BreakHitResult _array_element))))) (Variables|Default|GetTeamName))
      (bind _asbp_master_combat (Utilities|Casting|CastToBP_MasterCombat (.HitActor (Collision|BreakHitResult _array_element))))
      (Combat|DistressCall _asbp_master_combat (Variables|Combat|GetEnemyToFight))
      (return 0))))

(fn DistressCall
  (params (InEnemy :type Actor%20Object%20Reference))
  (return 0))

(fn OnDangerDetected
  (params (InActor :type Actor%20Object%20Reference))
  (Utilities|IsValid (Variables|Combat|GetEnemyToFight)
    (:Is%20Not%20Valid
      (bind _asbp_master_combat (Utilities|Casting|CastToBP_MasterCombat InActor)
        (:then
          (if (not (Utilities|Name|Equal(Name) (Variables|Default|GetTeamName) (Variables|/Game/MasterBlueprints/Units/BP_MasterUnit.BP_MasterUnit_C|GetTeamName _asbp_master_combat)))
            (Combat|OnSeeEnemies _asbp_master_combat)))
        (:CastFailed
          (bind _asbp_master_projectile (Utilities|Casting|CastToBP_MasterProjectile InActor))
          (Utilities|IsValid (Variables|/Game/MasterBlueprints/Items/BP_MasterProjectile.BP_MasterProjectile_C|GetFiredFrom _asbp_master_projectile)
            (:Is%20Valid
              (if (not (Utilities|Name|Equal(Name) (Variables|Default|GetTeamName) (Variables|/Game/MasterBlueprints/Units/BP_MasterUnit.BP_MasterUnit_C|GetTeamName (.AsBP%20Master%20Unit (Utilities|Casting|CastToBP_MasterUnit (Variables|/Game/MasterBlueprints/Items/BP_MasterProjectile.BP_MasterProjectile_C|GetFiredFrom _asbp_master_projectile))))))
                (Combat|OnSeeEnemies (Variables|/Game/MasterBlueprints/Items/BP_MasterProjectile.BP_MasterProjectile_C|GetFiredFrom _asbp_master_projectile))))))))))

(fn OnBumpbyFriendly
  (params (InBoxCollision :type Object%20Object%20Reference) (InActor :type Actor%20Object%20Reference))
  (bind _returnvalue (AI|GetBlackboard 0))
  (bind _enemytofight (Variables|Combat|GetEnemyToFight))
  (Utilities|Casting|CastToCapsuleComponent InBoxCollision)
  (if (Utilities|Name|Equal(Name) (Variables|Default|GetTeamName) (Variables|/Game/MasterBlueprints/Units/BP_MasterUnit.BP_MasterUnit_C|GetTeamName (.AsBP%20Master%20Unit (Utilities|Casting|CastToBP_MasterUnit InActor))))
    (if (Variables|Combat|GetOverrideAllOtherActions)
      (Utilities|IsValid _enemytofight
        (:Is%20Valid
          (bind _output_get (Variables|Combat|SetOverrideAllOtherActions false))
          (AI|Components|Blackboard|SetValueasBool _returnvalue (Variables|BBK|GetBBK_OverrideAllOtherActions) _output_get)))
      (else
        (Utilities|IsValid _enemytofight
          (:Is%20Not%20Valid
            _))))
    (Utilities|IsValid _returnvalue
      (:Is%20Valid
        (AI|Components|Blackboard|SetValueasBool _returnvalue (Variables|BBK|GetBBK_BumpMove) true)))))